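; Player camera pawn that zooms, pans and rotates a spring arm view, apparently for tactical play.
; Enhanced Input events update desired arm length (clamped), location (relative to the pawn's facing) and rotation (fixed yaw steps).
; Tick eases the arm and actor toward those targets with interpolation, using only X and Y for location.
; A helper adds the IMC_Tactical mapping context via a controller cast, but nothing here calls it.
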(event Input|EnhancedActionEvents|EnhancedInputActionIA_Zoom
  (params (ActionValue :type Float%20%28double-precision%29) (ElapsedSeconds :type Float%20%28double-precision%29) (TriggeredSeconds :type Float%20%28double-precision%29) (InputAction :type Input%20Action%20Object%20Reference :default "/Game/Input/Actions/IA_Zoom.IA_Zoom"))
  (CallFunction|CalculateZoom ActionValue))

(event Input|EnhancedActionEvents|EnhancedInputActionIA_Move
  (params (ActionValue :type Vector%202D%20Structure) (ElapsedSeconds :type Float%20%28double-precision%29) (TriggeredSeconds :type Float%20%28double-precision%29) (InputAction :type Input%20Action%20Object%20Reference :default "/Game/Input/Actions/IA_Move.IA_Move"))
  (CallFunction|CalculateMoveVector ActionValue))

(event Input|EnhancedActionEvents|EnhancedInputActionIA_Rotate
  (params (ActionValue :type Float%20%28double-precision%29) (ElapsedSeconds :type Float%20%28double-precision%29) (TriggeredSeconds :type Float%20%28double-precision%29) (InputAction :type Input%20Action%20Object%20Reference :default "/Game/Input/Actions/IA_Rotate.IA_Rotate"))
  (if (< ActionValue 0.0)
    (Variables|CameraRotation|SetRotation_Desired (Math|Rotator|CombineRotators (Variables|CameraRotation|GetRotation_Desired) (Math|Rotator|MakeRotator 0.0 0.0 (- 0.0 (Variables|CameraRotation|GetRotationSpeed)))))
    (else
      (Variables|CameraRotation|SetRotation_Desired (Math|Rotator|CombineRotators (Variables|CameraRotation|GetRotation_Desired) (Math|Rotator|MakeRotator 0.0 0.0 (Variables|CameraRotation|GetRotationSpeed)))))))

(event EventBeginPlay
  (CallFunction|SetInitialValues))

(event EventTick
  (params (DeltaSeconds :type Float%20%28single-precision%29))
  (CallFunction|ZoomCamera)
  (CallFunction|MoveCamera)
  (CallFunction|RotateCamera))

(fn ConstructionScript)

(fn BindEnhancedInputMapping
  (bind _asbp_player_character (Utilities|Casting|CastToBP_PlayerCharacter (Pawn|GetController)))
  (Input|AddMappingContext (PlayerController|LocalPlayerSubsystems|GetEnhancedInputLocalPlayerSubsystem _asbp_player_character) "/Game/Input/IMC_Tactical.IMC_Tactical" 0 "(bIgnoreAllPressedKeysUntilRelease=True,bForceImmediately=False,bNotifyUserSettings=False)"))

(fn CalculateZoom
  (params (Input :type Float%20%28double-precision%29))
  (Variables|CameraZoom|SetZoom_Desired (Math|Float|Clamp(Float) (+ (* Input (Variables|CameraZoom|GetZoom_ScrollSpeed)) (Variables|CameraZoom|GetZoom_Desired)) (Variables|CameraZoom|GetZoom_Min) (Variables|CameraZoom|GetZoom_Max))))

(fn SetInitialValues
  (Variables|CameraMovement|SetLocation_Desired (Transformation|GetActorLocation))
  (Variables|CameraZoom|SetZoom_Desired (Variables|/Script/Engine.SpringArmComponent|GetTargetArmLength (Variables|Default|GetSpringArm)))
  (Variables|CameraRotation|SetRotation_Desired "0, 0, 0"))

(fn ZoomCamera
  (Variables|/Script/Engine.SpringArmComponent|SetTargetArmLength (Variables|Default|GetSpringArm) (Math|Interpolation|FInterpTo (Variables|/Script/Engine.SpringArmComponent|GetTargetArmLength (Variables|Default|GetSpringArm)) (Variables|CameraZoom|GetZoom_Desired) (Utilities|Time|GetWorldDeltaSeconds) (Variables|CameraZoom|GetZoom_InterpSpeed))))

(fn MoveCamera
  (bind _returnvalue (Transformation|GetActorLocation))
  (bind _returnvalue_2 (Utilities|Time|GetWorldDeltaSeconds))
  (bind _location_desired (Variables|CameraMovement|GetLocation_Desired))
  (bind _location_interpspeed (Variables|CameraMovement|GetLocation_InterpSpeed))
  (bind _returnvalue_3 (Math|Interpolation|VInterpTo _returnvalue _location_desired _returnvalue_2 _location_interpspeed))
  (Transformation|SetActorLocation (Math|Vector|MakeVector (.x _returnvalue_3) (.y _returnvalue_3) 0.0) false false))

(fn CalculateMoveVector
  (params (MoveDir :type Vector%202D%20Structure))
  (bind _location_scrollspeed (Variables|CameraMovement|GetLocation_ScrollSpeed))
  (Variables|CameraMovement|SetLocation_Desired (+ (+ (Math|Vector|MakeVector (.x (Variables|CameraMovement|GetLocation_Desired)) 0.0 0.0) (* (Transformation|GetActorForwardVector) (* (.x MoveDir) _location_scrollspeed))) (+ (Math|Vector|MakeVector 0.0 (.y (Variables|CameraMovement|GetLocation_Desired)) 0.0) (* (* (.y MoveDir) _location_scrollspeed) (Transformation|GetActorRightVector))))))

(fn RotateCamera
  (Transformation|SetActorRotation (Math|Interpolation|RInterpTo (Transformation|GetActorRotation) (Variables|CameraRotation|GetRotation_Desired) (Utilities|Time|GetWorldDeltaSeconds) (Variables|CameraRotation|GetRotation_InterpSpeed))))